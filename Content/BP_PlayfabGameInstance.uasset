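; PlayFab game instance that handles player account sign-up, email login and password recovery, setting the title ID on Init.
; SignUp, LogIn and ForgotPassword each send a PlayFab client request with success and failure callbacks.
; Successful registration or login opens the main menu level, while a sent recovery email prints a confirmation.
; OnFail prints registration error details to screen in red.
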(event `self.ReceiveInit`
  (`PlayFabUtilities.setPlayFabSettings` (`self.GameId`)))

(event `OnRegisterSuccess`
  (params (result :type "ClientRegisterPlayFabUserResult Structure") (customData :type "Object Object Reference"))
  ;[1 1 1] Sign Up
  (`GameplayStatics.OpenLevelBySoftObjectPtr` "/Game/LVL_MainMenu.LVL_MainMenu"))

(event `SignUp`
  (params (Username :type String) (EMail :type String) (Password :type String))
  ;[1 1 1] Sign Up
  (`PlayFabClientAPI.RegisterPlayFabUser` (make `ClientRegisterPlayFabUserRequest` null Username EMail "" null Password "" false Username) (delegate `OnRegisterSuccess`) (delegate `OnFail`)))

(event `OnFail`
  (params (error :type "PlayFabError Structure") (customData :type "Object Object Reference"))
  (bind (_haserror _errorcode _errorname _errormessage _errordetails) (break `PlayFabError` error))
  (`KismetSystemLibrary.PrintString` (`KismetStringLibrary.Concat_StrStr` _errorname "(" _errormessage " - " _errordetails ")") true true (struct :`R` 1.0 :`B` 0.053995 :`A` 1.0)))

(event `LogIn`
  (params (EMail :type String) (Password :type String))
  ;[1 1 1] Log In
  (`PlayFabClientAPI.LoginWithEmailAddress` (make `ClientLoginWithEmailAddressRequest` null EMail null Password) (delegate `OnLogInSuccess`) (`|CreateDelegate` :!event `OnFail`)))

(event `OnLogInSuccess`
  (params (result :type "ClientLoginResult Structure") (customData :type "Object Object Reference"))
  ;[1 1 1] Log In
  (`GameplayStatics.OpenLevelBySoftObjectPtr` "/Game/LVL_MainMenu.LVL_MainMenu"))

(event `RecoveryEmailSuccess`
  (params (result :type "ClientSendAccountRecoveryEmailResult Structure") (customData :type "Object Object Reference"))
  ;[1 0.374 0.4635] Recovery
  (`KismetSystemLibrary.PrintString` "Recovery mail sent" true true (struct :`R` 0.266062 :`G` 1.0 :`A` 1.0)))

(event `ForgotPassword`
  (params (EMail :type String))
  ;[1 0.374 0.4635] Recovery
  (`PlayFabClientAPI.SendAccountRecoveryEmail` (make `ClientSendAccountRecoveryEmailRequest` null EMail) (delegate `RecoveryEmailSuccess`) (`|CreateDelegate` :!event `OnFail`)))